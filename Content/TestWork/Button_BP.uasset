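; Pressure-plate button Blueprint that sinks and lights a lamp while third-person characters stand on its trigger box.
; An overlap counter drives a timeline that lowers the actor from its start location and reverses once nobody remains.
; A second timeline animates the point light and the sphere's dynamic material, blending its color track with a Color variable.
; When the plate empties, that timeline stops and both turn black.
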(event `self.ReceiveBeginPlay`
  ;[1 1 1] Begin Play - save actor start location; creating dynamic material
  (set `self.StartVector` (`self.K2_GetActorLocation`))
  (bind _returnvalue (`PrimitiveComponent.CreateDynamicMaterialInstance` (`self.Sphere`) 0 "/Game/TestWork/Lamp_M_Inst.Lamp_M_Inst" "None"))
  (set `self.Dynamic_M` _returnvalue))

(event `self.Box.OnComponentBeginOverlap`
  (params (OverlappedComponent :type "PrimitiveComponent Object Reference") (OtherActor :type "Actor Object Reference") (OtherComp :type "PrimitiveComponent Object Reference") (OtherBodyIndex :type Integer) (bFromSweep :type Boolean) (SweepResult :type "HitResult Structure (by ref)"))
  ;[1 1 1] Trigger Begin Overlap - calculating count of player on platform; enable platform moving down; enable lamp light
  (cast `/Game/ThirdPersonCPP/Blueprints/ThirdPersonCharacter` OtherActor)
  (`/Engine/EditorBlueprintResources/StandardMacros.IncrementInt` (`self.PlayersOnPlatform`)
    (:`  `
      (`self.MoveDown`)
      (`self.EnableLight`))))

(event `self.Box.OnComponentEndOverlap`
  (params (OverlappedComponent :type "PrimitiveComponent Object Reference") (OtherActor :type "Actor Object Reference") (OtherComp :type "PrimitiveComponent Object Reference") (OtherBodyIndex :type Integer))
  (bind _playersonplatform (`self.PlayersOnPlatform`))
  ;[1 1 1] Trigger End Overlap - calculating count of player on platform; if players on platform 0 - disable platform moving down, disable lamp light
  (cast `/Game/ThirdPersonCPP/Blueprints/ThirdPersonCharacter` OtherActor)
  (`/Engine/EditorBlueprintResources/StandardMacros.DecrementInt` _playersonplatform
    (:`  `
      (if (< _playersonplatform 1)
        (`self.MoveUp`)
        (`self.DisableLight`)))))

(event `MoveDown`
  ;[1 1 1] Move platform down
  ;[1 1 1] Platform moving
  (bind (_direction _highvalue) (`Timeline|MovePlatformDown` :!label _label)
    (:`Update`
      (`self.K2_SetActorLocation` (`KismetMathLibrary.MakeVector` (.x (`self.StartVector`)) (.y (`self.StartVector`)) (- (.z (`self.StartVector`)) (* _highvalue 20.0)))))))

(event `MoveUp`
  ;[1 1 1] Move platform up
  (goto _label :!via `Reverse`))

(event `DisableLight`
  ;[1 1 1] Disable Light - disable lamp color changing, set point light color for BLACK, set sphere color for BLACK
  (`self.StopLampColor`)
  (`LightComponent.SetLightColor` :`self` (`self.PointLight`))
  (`MaterialInstanceDynamic.SetVectorParameterValue` :`self` (`self.Dynamic_M`) :`ParameterName` "Color"))

(event `EnableLight`
  ;[1 1 1] Enable Light - enable lamp color changing, set point light color for WHITE
  (`self.ChangeLampColor`)
  (`LightComponent.SetLightColor` (`self.PointLight`) (struct :`R` 1.0 :`G` 1.0 :`B` 1.0 :`A` 1.0) true))

(event `ChangeLampColor`
  ;[1 1 1] Enable color changing
  ;[1 1 1] Lamp Color Changing
  (bind (_direction _color) (`Timeline|ChangeColor` :!label _label_2)
    (:`Update`
      (bind _returnvalue (`KismetMathLibrary.LinearColorLerp` _color (`self.Color`) 0.7))
      (`MaterialInstanceDynamic.SetVectorParameterValue` (`self.Dynamic_M`) "Color" _returnvalue)
      (`LightComponent.SetLightColor` (`self.PointLight`) _returnvalue true))))

(event `StopLampColor`
  ;[1 1 1] Disable color changing
  (goto _label_2 :!via `Stop`))

(fn `UserConstructionScript`)